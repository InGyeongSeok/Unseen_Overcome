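; BP_OVCharacterPlayer is a player character Blueprint that toggles a sphere component, apparently tied to a shield skill.
; Every Tick it checks IsActiveShieldSkill: when true the Sphere is hidden with collision off, otherwise it is visible with query and physics collision as a Pawn object.
; An outline overlay material call in the construction script is disconnected, and the teleport skill flag is unused.
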(event `self.ReceiveTick`
  (params (DeltaSeconds :type "Float (single-precision)"))
  (if (`self.bIsActiveShieldSkill`)
    (`SceneComponent.SetVisibility` (`self.Sphere`) false false)
    (`PrimitiveComponent.SetCollisionEnabled` (`self.Sphere`) "NoCollision")
    (`PrimitiveComponent.SetCollisionObjectType` (`self.Sphere`) "ECC_Pawn")
    (else
      (`SceneComponent.SetVisibility` (`self.Sphere`) true false)
      (`PrimitiveComponent.SetCollisionEnabled` (`self.Sphere`) "QueryAndPhysics")
      (`PrimitiveComponent.SetCollisionObjectType` (`self.Sphere`) "ECC_Pawn"))))

(fn `UserConstructionScript`)